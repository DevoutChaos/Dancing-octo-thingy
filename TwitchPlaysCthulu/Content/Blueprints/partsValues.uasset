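; partsValues is a lookup Blueprint that holds per-position values for five elemental monster types: Fire, Air, Water, Lightning and Earth.
; GetValue switches on the Monster type and returns the entry at the given Position from that element's own array.
; The construction script is empty, and the array contents are not set in the graphs.
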(fn `getValue`
  (params (monster :type String) (position :type Integer))
  (returns (value :type Integer))
  (switch `string` monster
    (:`Fire`
      ;[1 1 1] fire
      (return (`KismetArrayLibrary.Array_Get` (`self.FireMonstValues`) position)))
    (:`Air`
      ;[1 1 1] Air
      (return (`KismetArrayLibrary.Array_Get` (`self.AirMonstValues`) position)))
    (:`Water`
      ;[1 1 1] Water
      (return (`KismetArrayLibrary.Array_Get` (`self.WaterMonstValues`) position)))
    (:`Lightning`
      ;[1 1 1] Lightning
      (return (`KismetArrayLibrary.Array_Get` (`self.LightningMonstValues`) position)))
    (:`Earth`
      ;[1 1 1] Earth
      (return (`KismetArrayLibrary.Array_Get` (`self.EarthMonstValues`) position)))))

(fn `UserConstructionScript`)