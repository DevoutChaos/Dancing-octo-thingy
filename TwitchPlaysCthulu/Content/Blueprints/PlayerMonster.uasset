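; Player monster Blueprint that assembles a monster part by part and takes damage reduced by DamResistance.
; Each appPart call shows the element's sprite for the current slot, overwrites Health from a Values lookup by type and slot, then advances the slot.
; Completing the fifth part tells EnemyMonst to create its monster.
; Fire, Earth and Water are wired; Lightning and Air branches are unfinished.
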(event `EnemyTakeDamage`
  (params (Damage :type Integer))
  ;[1 1 1] damage call
  (set `self.health` (- (`self.health`) (/ Damage (`self.DamResistance`)))))

(event `appPart`
  (params (monstName :type String))
  (bind _partno (`self.partNo`))
  (bind _values (`self.values`))
  (bind _monst_type (`self.monst type`))
  (bind _partno_2 (`self.partNo`))
  (bind _output_get (set `self.monst type` monstName))
  (switch `string` _output_get
    (:`Fire`
      (switch `int` _partno ; fire sprite selection
        (:`0`
          ;[1 1 1] 1-body, 2-head, 3-arms, 4-legs, 5-other
          (`SceneComponent.SetVisibility` (`self.fire body_Sprite`) true true)
          ;[1 1 1] grab values
          (bind _value (`/Game/Blueprints/partsValues.getValue` _values _monst_type _partno_2 :!label _label))
          (set `self.health` _value))
        (:`1`
          (`SceneComponent.SetVisibility` (`self.fire head_Sprite`) true true)
          (bind _value_2 (`/Game/Blueprints/partsValues.getValue` _values _monst_type _partno_2 :!label _label_2))
          (set `self.health` _value_2))
        (:`2`
          (`SceneComponent.SetVisibility` (`self.fire arms_Sprite`) true true)
          (bind _value_3 (`/Game/Blueprints/partsValues.getValue` _values _monst_type _partno_2 :!label _label_3))
          (set `self.health` _value_3))
        (:`3`
          (`SceneComponent.SetVisibility` (`self.fire legs_Sprite`) true true)
          (bind _value_4 (`/Game/Blueprints/partsValues.getValue` _values _monst_type _partno_2 :!label _label_4))
          (set `self.health` _value_4))
        (:`4`
          (`SceneComponent.SetVisibility` (`self.fire tail_Sprite`) true true)
          (`SceneComponent.SetVisibility` (`self.fire wings_Sprite`) true true)
          (bind _value_5 (`/Game/Blueprints/partsValues.getValue` _values _monst_type _partno_2 :!label _label_5))
          (set `self.health` _value_5)))
      (bind _result (`/Engine/EditorBlueprintResources/StandardMacros.IncrementInt` (`self.partNo`))
        (:`  `
          (bind _output_get_2 (set `self.partNo` _result))
          (if (== _output_get_2 5)
            (`/Game/Blueprints/EnemyMonster.createMonster` (`self.enemyMonst`))))))
    (:`Earth`
      (switch `int` _partno ; earth sprite selection
        (:`0`
          ;[1 1 1] 1-body, 2-head, 3-arms, 4-legs, 5-other
          (`SceneComponent.SetVisibility` (`self.earth body_Sprite`) true true)
          (goto _label))
        (:`1`
          (`SceneComponent.SetVisibility` (`self.earth head_Sprite`) true true)
          (goto _label_2))
        (:`2`
          (`SceneComponent.SetVisibility` (`self.earth arms_Sprite`) true true)
          (goto _label_3))
        (:`3`
          (`SceneComponent.SetVisibility` (`self.earth legs_Sprite`) true true)
          (goto _label_4))
        (:`4`
          (`SceneComponent.SetVisibility` (`self.earth wings_Sprite`) true true)
          (goto _label_5))))
    (:`Water`
      (switch `int` _partno ; fire sprite selection
        (:`0`
          ;[1 1 1] 1-body, 2-head, 3-arms, 4-legs, 5-other
          (`SceneComponent.SetVisibility` (`self.water head_Sprite`) true true)
          (goto _label))
        (:`1`
          (`SceneComponent.SetVisibility` (`self.water horns_Sprite`) true true)
          (goto _label_2))
        (:`2`
          (`SceneComponent.SetVisibility` (`self.water back_tentacles_Sprite`) true true)
          (goto _label_3))
        (:`3`
          (`SceneComponent.SetVisibility` (`self.water legs_front_Sprite`) true true)
          (goto _label_4))
        (:`4`
          (`SceneComponent.SetVisibility` (`self.water legs_mid_Sprite`) true true)
          (`SceneComponent.SetVisibility` (`self.water legs_back_Sprite`) true true)
          (goto _label_5))))
    (:`Lightning`
      (switch `int` _partno) ; lightning sprite selection
    )
    (:`Air`
      (switch `int` _partno) ; air sprite selection
    )))

(fn `UserConstructionScript`)