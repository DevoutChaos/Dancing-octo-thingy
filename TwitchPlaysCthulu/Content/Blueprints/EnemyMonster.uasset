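; Enemy monster actor that fights the player's monster in timed combat and, on death, triggers the player win and reloads the main level.
; createMonster shows five body-part sprites, pulls health, resistance, damage and crit chance from Values, then starts combat and the player UI.
; Only the fire set is wired; random element selection is disconnected.
; Tick drives cooldown-gated attacks with double-damage crits, while incoming damage is divided by resistance.
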(event `EnemyTakeDamage`
  (params (Damage :type Integer))
  ;[1 1 1] damage call
  (bind _output_get (set `self.EnemyHealth` (- (`self.EnemyHealth`) (/ Damage (`self.damResis`)))))
  ;[1 1 1] death call
  (if (<= _output_get 0)
    (`KismetSystemLibrary.PrintString` "player kills monster")
    (`/Game/Blueprints/GOCondition.PlayerWin` (`self.GOCondition`))
    (`self.K2_DestroyActor`)
    (`GameplayStatics.OpenLevel` "mainLevelBPfixes")
    (else
      (`KismetSystemLibrary.PrintString` "player hits monster"))))

(event `self.ReceiveTick`
  (params (DeltaSeconds :type "Float (single-precision)"))
  (bind _damage (`self.damage`))
  (bind _playermonst (`self.playerMonst`))
  (if (`self.CombatTime`)
    (if (`self.EnemyCanAttack`)
      (set `self.EnemyCanAttack` false)
      ;[1 1 1] crit  attack]
      (if (<= (`KismetMathLibrary.RandomIntegerInRange` 0 100) (`self.critChance`))
        (`/Game/Blueprints/PlayerMonster.EnemyTakeDamage` _playermonst (* _damage 2))
        (else
          (`/Game/Blueprints/PlayerMonster.EnemyTakeDamage` _playermonst _damage)))
      (else
        (`KismetSystemLibrary.Delay` (stale `self.ReceiveBeginPlay` _output_get))
        (set `self.EnemyCanAttack` true)))))

(event `self.ReceiveBeginPlay`
  (set `self.CombatTime` false)
  (bind _output_get (set `self.EnemyCooldown` (`self.EnemyCooldown`))))

(event `createMonster`
  (bind _values (`self.values`))
  (bind _damage (`self.damage`))
  (bind _i (`self.i`))
  (for _index (range 5)
    (set `self.i` _index)
    (switch `int` _index ; fire sprite selection
      (:`0`
        ;[1 1 1] 1-body, 2-head, 3-arms, 4-legs, 5-other
        (`SceneComponent.SetVisibility` (`self.fire body_Sprite`) true true)
        ;[1 1 1] grab values
        (bind _value (`/Game/Blueprints/partsValues.getValue` _values "" (`self.randNum`)))
        (bind _output_get (set `self.EnemyHealth` _value))
        (set `self.maxHealth` _output_get))
      (:`1`
        (`SceneComponent.SetVisibility` (`self.fire head_Sprite`) true true)
        (bind _value_2 (`/Game/Blueprints/partsValues.getValue` _values "" _i))
        (set `self.damResis` _value_2))
      (:`2`
        (`SceneComponent.SetVisibility` (`self.fire arms_Sprite`) true true)
        (bind _value_3 (`/Game/Blueprints/partsValues.getValue` _values "" _i))
        (set `self.damage` (+ _value_3 _damage)))
      (:`3`
        (`SceneComponent.SetVisibility` (`self.fire legs_Sprite`) true true)
        (bind _value_4 (`/Game/Blueprints/partsValues.getValue` _values "" _i))
        (set `self.damage` (+ _damage _value_4)))
      (:`4`
        (`SceneComponent.SetVisibility` (`self.fire tail_Sprite`) true true)
        (bind _value_5 (`/Game/Blueprints/partsValues.getValue` _values "" _i))
        (set `self.critChance` _value_5))))
  (`KismetSystemLibrary.PrintString` "FIGHT")
  (set `self.CombatTime` true)
  (`/Game/Blueprints/PlayerMonster.start UI` (`self.playerMonst`)))

(fn `getPercentageHP`
  (returns (percent :type "Float (double-precision)"))
  (return (/ (`KismetMathLibrary.Conv_IntToDouble` (`self.maxHealth`)) (`KismetMathLibrary.Conv_IntToDouble` (`self.EnemyHealth`)))))

(fn `UserConstructionScript`)